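; Enemy spawner that produces random enemies from a class list while the Planet game mode has a wave in play.
; Tick caches the game mode and, the first time PlayWave is true, starts a looping sub-second timer through a DoOnce.
; Each timer call rechecks PlayWave, increments the game mode's enemy count, then spawns a random class at a stored transform.
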(event `SpawnEnemy`
  (if (`/Game/Planet_GameMode.PlayWave` (stale _asplanet_game_mode))
    (`|ExecutionSequence`
      (:`then_0`
        (bind _asplanet_game_mode (cast `/Game/Planet_GameMode` (`GameplayStatics.GetGameMode`)))
        (set `/Game/Planet_GameMode.NumberOfEnemies` (+ (`/Game/Planet_GameMode.NumberOfEnemies` _asplanet_game_mode) 1) _asplanet_game_mode))
      (:`then_1`
        (`|SpawnActorFromClass` (`self.GetRandomEnemy`) (`self.NewVar_0`) "Undefined" "OverrideRootScale" null null)))))

(event `self.ReceiveTick`
  (params (DeltaSeconds :type "Float (single-precision)"))
  (`|ExecutionSequence`
    (:`then_0`
      (if (`/Game/Planet_GameMode.PlayWave` (stale _asplanet_game_mode))
        (`/Engine/EditorBlueprintResources/StandardMacros.DoOnce` false
          (:`Completed`
            (`KismetSystemLibrary.K2_SetTimerDelegate` (delegate `SpawnEnemy`) 0.8 true)))))
    (:`then_1`
      (bind _asplanet_game_mode (cast `/Game/Planet_GameMode` (`GameplayStatics.GetGameMode`))))))

(fn `GetRandomEnemy`
  (returns (Enemy :type "/Game/Blueprints/BP_Enemy Class Reference"))
  (bind _enemyclasses (`self.EnemyClasses`))
  (return (`|GetArrayItem` _enemyclasses (`KismetMathLibrary.RandomIntegerInRange` 0 (- (`KismetArrayLibrary.Array_Length` _enemyclasses) 1)))))

(fn `UserConstructionScript`)