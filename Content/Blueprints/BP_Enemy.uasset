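; BP_Enemy is an enemy actor that travels along a spline and is killed by any actor overlap.
; On the first Tick, it sets a random yaw, rotating its path, then plays a timeline that drives MoveOnSpline to place EnemyMesh by normalized spline distance.
; On overlap, it decrements the enemy count in Planet_GameMode, prints a message, spawns BP_Explosion at the mesh and destroys itself.
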(event `self.ReceiveActorBeginOverlap`
  (params (OtherActor :type "Actor Object Reference"))
  (`|ExecutionSequence`
    (:`then_0`
      (bind _asplanet_game_mode (cast `/Game/Planet_GameMode` (`GameplayStatics.GetGameMode`)))
      (set `/Game/Planet_GameMode.NumberOfEnemies` (- (`/Game/Planet_GameMode.NumberOfEnemies` _asplanet_game_mode) 1) _asplanet_game_mode))
    (:`then_1`
      (`KismetSystemLibrary.PrintString` "Enemy has been killed")
      (`|SpawnActorFromClass` "/Game/Blueprints/bp_Explosion.BP_Explosion_C" (`SceneComponent.K2_GetComponentToWorld` (`self.EnemyMesh`)) "Undefined" "OverrideRootScale" null null)
      (`self.K2_DestroyActor`))))

(event `self.ReceiveTick`
  (params (DeltaSeconds :type "Float (single-precision)"))
  (`/Engine/EditorBlueprintResources/StandardMacros.DoOnce` false
    (:`Completed`
      (`self.K2_SetActorRotation` (`KismetMathLibrary.MakeRotator` 0.0 0.0 (`KismetMathLibrary.RandomFloatInRange` 0.0 359.9)))
      (bind (_direction _enemytraveltime_01) (`Timeline|Timeline_0` :!via `PlayFromStart`)
        (:`Update`
          (`self.MoveOnSpline` _enemytraveltime_01))))))

(fn `MoveOnSpline`
  (params (ZicZac :type "Float (double-precision)") (Direct :type "Float (double-precision)"))
  (bind _spline (`self.Spline`))
  (bind _returnvalue (* (`SplineComponent.GetSplineLength` _spline) ZicZac))
  (`SceneComponent.K2_SetWorldTransform` (`self.EnemyMesh`) (`KismetMathLibrary.MakeTransform` (`SplineComponent.GetLocationAtDistanceAlongSpline` _spline _returnvalue "World") (`SplineComponent.GetRotationAtDistanceAlongSpline` _spline _returnvalue "World")) false false))

(fn `UserConstructionScript`)