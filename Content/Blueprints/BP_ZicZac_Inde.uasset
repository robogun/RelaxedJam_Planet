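; BP_ZicZac_Inde is an actor that carries an enemy mesh along a spline, apparently a zigzag path.
; On the first Tick, a DoOnce gives the actor a random yaw, so the path points in a random direction, then plays ZicZacTimeLine.
; Each timeline update feeds MovingOnSpline, which scales the value by spline length and sets EnemyMesh's world location and rotation from that point.
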(event `self.ReceiveTick`
  (params (DeltaSeconds :type "Float (single-precision)"))
  (`/Engine/EditorBlueprintResources/StandardMacros.DoOnce` false
    (:`Completed`
      (`self.K2_SetActorRotation` (`KismetMathLibrary.MakeRotator` 0.0 0.0 (`KismetMathLibrary.RandomFloatInRange` 0.0 359.9)))
      (bind (_direction _ziczac_traveltime) (`Timeline|ZicZacTimeLine`)
        (:`Update`
          (`self.MovingOnSpline` _ziczac_traveltime))))))

(fn `MovingOnSpline`
  (params (ZicZac_Speed :type "Float (double-precision)"))
  (bind _spline (`self.Spline`))
  (bind _returnvalue (* (`SplineComponent.GetSplineLength` _spline) ZicZac_Speed))
  (`SceneComponent.K2_SetWorldTransform` (`self.EnemyMesh`) (`KismetMathLibrary.MakeTransform` (`SplineComponent.GetLocationAtDistanceAlongSpline` _spline _returnvalue "World") (`SplineComponent.GetRotationAtDistanceAlongSpline` _spline _returnvalue "World")) false false))

(fn `UserConstructionScript`
  (`parent.UserConstructionScript`))